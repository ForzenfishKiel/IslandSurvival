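; Wooden door actor for the building system that swings open away from or toward closed when interacted with.
; The interact event calls OpenDoorOnMult, which plays a timeline that yaws the mesh up to 90 degrees, choosing the side from a dot product of the interactor's position and the door's forward vector.
; Further interactions reverse the timeline, and the door counts as closed again only when the reverse finishes.
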(event `self.ReceiveTick`
  (params (DeltaSeconds :type "Float (single-precision)"))
  (`parent.ReceiveTick` DeltaSeconds))

(event `ISBuildInterface.OnBuildingWasInteract`
  (params (InteractingActor :type "Actor Object Reference") (InteractingComponent :type "ActorComponent Object Reference"))
  (`self.OpenDoorOnMult` InteractingActor InteractingComponent))

(event `OpenDoorOnMult`
  (params (InActor :type "Actor Object Reference") (InComponent :type "ActorComponent Object Reference"))
  (bind _rootscenecomponent (`self.RootSceneComponent`))
  (if (`self.IsDoorClosed`)
    (set `self.IsDoorClosed` false)
    (set `self.DotProDuct` (`KismetMathLibrary.Dot_VectorVector` (`KismetMathLibrary.Normal` (- (`SceneComponent.K2_GetComponentLocation` _rootscenecomponent) (`self.K2_GetActorLocation` InActor))) (`SceneComponent.GetForwardVector` _rootscenecomponent)))
    (bind (_direction __alpha) (`Timeline|OpenDoorTL` :!label _label)
      (:`Update`
        (`SceneComponent.K2_SetRelativeRotation` (`self.ItemsStaticMesh`) (`KismetMathLibrary.MakeRotator` 0.0 0.0 (`KismetMathLibrary.Lerp` 0.0 (`KismetMathLibrary.SelectFloat` 90.0 -90.0 (>= (`self.DotProDuct`) 0.0)) __alpha)) false false))
      (:`Finished`
        (switch `ETimelineDirection` _direction
          (:`Backward`
            (set `self.IsDoorClosed` true)))))
    (else
      (goto _label :!via `Reverse`))))

(fn `UserConstructionScript`
  (`parent.UserConstructionScript`))