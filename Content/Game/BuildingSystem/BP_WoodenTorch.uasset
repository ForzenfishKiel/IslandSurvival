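; BP_WoodenTorch is a wooden torch for the building system that players can light or put out by interacting with it.
; OnBuildingWasInteract toggles the IsTorchLit flag, whose RepNotify sets the visibility of the PTorchFire component to match.
; The replicated flag keeps the flame in sync across the network, with no Tick logic.
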(event `ISBuildInterface.OnBuildingWasInteract`
  (params (InteractingActor :type "Actor Object Reference") (InteractingComponent :type "ActorComponent Object Reference"))
  (if (`self.IsTorchLit`)
    (set `self.IsTorchLit` false)
    (else
      (set `self.IsTorchLit` true))))

(fn `OnRep_IsTorchLit`
  (`SceneComponent.SetVisibility` (`self.P_TorchFire`) (`self.IsTorchLit`) false))

(fn `UserConstructionScript`
  (`parent.UserConstructionScript`))