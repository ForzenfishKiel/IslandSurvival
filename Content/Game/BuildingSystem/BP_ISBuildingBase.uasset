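; Base actor for building-system pieces that handles a piece breaking apart.
; EnableBuildBroken checks that the target actor is valid, then calls MulticastEvryone, which swaps the intact mesh for a physics-simulated destructible mesh.
; That event also spawns a BP_DestroySystem with a resized sphere at the piece's location and sets a short lifespan for cleanup.
; DestorySnappeStructs is an empty stub here.
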(event `self.EnableBuildBroken`
  (params (TargetActor :type "Actor Object Reference"))
  (`/Engine/EditorBlueprintResources/StandardMacros.IsValid` TargetActor
    (:`Is Valid`
      (`self.MulticastEvryone`))))

(event `MulticastEvryone`
  (bind _itemsstaticmesh (`self.ItemsStaticMesh`))
  (bind _destructblemesh (`self.DestructbleMesh`))
  (`PrimitiveComponent.SetCollisionEnabled` _itemsstaticmesh "NoCollision")
  (`SceneComponent.SetVisibility` _itemsstaticmesh false false)
  (`SceneComponent.SetVisibility` _destructblemesh true false)
  (`PrimitiveComponent.SetSimulatePhysics` _destructblemesh true)
  (bind _returnvalue (`|SpawnActorFromClass` "/Game/Game/Havestion/BP_DestroySystem.BP_DestroySystem_C" (`KismetMathLibrary.MakeTransform` (`self.K2_GetActorLocation`)) "Undefined" "MultiplyWithRoot" null null))
  (`SphereComponent.SetSphereRadius` (`/Game/Game/Havestion/BP_DestroySystem.Sphere` _returnvalue) 200.0 true)
  (`self.SetLifeSpan` 8.0))

(fn `DestorySnappeStructs`
  (params (InActor :type "Actor Object Reference")))

(fn `UserConstructionScript`)