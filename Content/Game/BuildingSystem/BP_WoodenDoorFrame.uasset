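; BP_WoodenDoorFrame is a wooden door frame piece in the building system that passes breakage on to nearby structures.
; It extends the parent's EnableBuildBroken event by calling DestorySnappeStructs after the parent logic.
; That event gathers actors overlapping the DestorySearch component and sends DestoryBuildingMessage, with the target actor, to those implementing ISBuildInterface.
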(event `self.EnableBuildBroken`
  (params (TargetActor :type "Actor Object Reference"))
  (`parent.EnableBuildBroken` TargetActor)
  (`self.DestorySnappeStructs` TargetActor))

(event `self.DestorySnappeStructs`
  (params (InActor :type "Actor Object Reference"))
  (bind _overlappingactors (`PrimitiveComponent.GetOverlappingActors` (`self.DestorySearch`) null))
  (if (`KismetArrayLibrary.Array_IsNotEmpty` _overlappingactors)
    (for _array_element _overlappingactors
      (if (`KismetSystemLibrary.DoesImplementInterface` _array_element "/Script/IslandSurvival.ISBuildInterface")
        (message `ISBuildInterface.DestoryBuilding` _array_element InActor)))))

(fn `UserConstructionScript`
  (`parent.UserConstructionScript`))