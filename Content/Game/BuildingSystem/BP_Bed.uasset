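; BP_Bed is a placeable bed in the building system that sets a player's respawn point.
; When interacted with, it passes its own location to the interacting actor through SetPlayerRespawnLocationMessage, an interface-style message call.
; It then prints an on-screen confirmation in Chinese that the respawn point is set.
; Its other events are disabled stubs and the construction script only calls the parent.
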(event `ISBuildInterface.OnBuildingWasInteract`
  (params (InteractingActor :type "Actor Object Reference") (InteractingComponent :type "ActorComponent Object Reference"))
  ;[0 0.4215 1] 玩家与床交互以后设置重生点
  (message `ISPlayerInterface.SetPlayerRespawnLocation` InteractingActor (`self.K2_GetActorLocation`))
  (`KismetSystemLibrary.PrintString` "已设置重生点" true true (struct :`R` 1.0 :`G` 0.15107 :`A` 1.0) 10.0))

(fn `UserConstructionScript`
  (`parent.UserConstructionScript`))