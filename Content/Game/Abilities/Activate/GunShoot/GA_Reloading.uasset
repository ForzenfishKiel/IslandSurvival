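; Gameplay ability that reloads the player's equipped gun by consuming a magazine from the hotbar inventory.
; It checks through BP_GunsInterface that ammo is below maximum and a magazine check passes, then plays the rifle reload montage on the arm mesh.
; On completion, only the authority discards one magazine, refills ammo and ends the ability.
; Failed checks (except the player cast) and montage interruption also end it.
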(event `self.K2_ActivateAbility`
  (bind _asbp_ismain_player (cast `/Game/Game/Character/BP_ISMainPlayer` (`self.GetAvatarActorFromActorInfo`) :!label _label))
  (bind _equipable (`ISEquipmentComponent.Equipable` (`Actor.GetComponentByClass` _asbp_ismain_player "/Script/IslandSurvival.ISEquipmentComponent")))
  (if (`KismetSystemLibrary.DoesImplementInterface` _equipable "/Game/Game/BlueprintInterface/BP_GunsInterface.BP_GunsInterface_C")
    (bind _ammos (message `/Game/Game/BlueprintInterface/BP_GunsInterface.GetAmmos` _equipable))
    (bind _outmaxammo (message `/Game/Game/BlueprintInterface/BP_GunsInterface.Get MaxAmmo` _equipable))
    (if (< _ammos _outmaxammo)
      (bind _havemagazine (message `/Game/Game/BlueprintInterface/BP_GunsInterface.CallCheckMagazine` _equipable))
      (if _havemagazine
        (`|PlayMontage` (`ISCharacter.ArmMesh` _asbp_ismain_player) "/Game/Game/Animations/Locomotion/Rifle/AM_RifleReload.AM_RifleReload"
          (:`OnCompleted`
            (`self.K2_HasAuthority`
              (:`True`
                (bind _outindex (message `/Game/Game/BlueprintInterface/BP_GunsInterface.GetMagazineIndex` _equipable))
                (if (!= _outindex -1)
                  (`ISItemsContainer.DiscardItem` (`Actor.GetComponentByClass` _asbp_ismain_player "/Script/IslandSurvival.ISHotBarInventory") _outindex 1)
                  (message `/Game/Game/BlueprintInterface/BP_GunsInterface.FullAmmo` _equipable)
                  (`self.K2_EndAbility`)
                  (else
                    (`self.K2_EndAbility`))))))
          (:`OnInterrupted`
            (`self.K2_EndAbility`)))
        (else
          (`self.K2_EndAbility`)))
      (else
        (`self.K2_EndAbility`)))
    (else
      (`self.K2_EndAbility`))))

(event `self.K2_ActivateAbilityFromEvent`
  (params (EventData :type "GameplayEventData Structure (by ref)"))
  (goto _label))