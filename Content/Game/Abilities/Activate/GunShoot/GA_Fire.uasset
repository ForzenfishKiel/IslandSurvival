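; Gameplay ability that fires the player's equipped item, ending at once if it has no ammo.
; It plays the item's first activate montage at double rate on the arm mesh and, in parallel, through a PlayMontageAndWait task.
; The arm montage's notify tells the item to open fire and commit ammo, on authority only.
; Completion of either montage ends the ability, while a missing item or empty animation list leaves it without an EndAbility call.
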(event `self.K2_ActivateAbility`
  (bind _asbp_ismain_player (cast `/Game/Game/Character/BP_ISMainPlayer` (`self.GetAvatarActorFromActorInfo`)))
  (bind _equipable (`ISEquipmentComponent.Equipable` (`Actor.GetComponentByClass` _asbp_ismain_player "/Script/IslandSurvival.ISEquipmentComponent"))
    (:`then`
      (bind _ammos (message `/Game/Game/BlueprintInterface/BP_GunsInterface.GetAmmos` _equipable))
      (if (<= _ammos 0)
        (`self.K2_EndAbility`)
        (else
          (bind _equipableactivateanimations (`ISEquipable.EquipableActivateAnimations` _equipable))
          (if (not (`KismetArrayLibrary.Array_IsEmpty` _equipableactivateanimations))
            (`|ExecutionSequence`
              (:`then_0`
                (bind _output (`|GetArrayItem` _equipableactivateanimations))
                (`|PlayMontage` (`ISCharacter.ArmMesh` _asbp_ismain_player) _output 2.0
                  (:`OnCompleted`
                    (`self.K2_EndAbility` :!label _label))
                  (:`OnNotifyBegin`
                    (`self.K2_HasAuthority`
                      (:`True`
                        (message `/Game/Game/BlueprintInterface/BP_GunsInterface.OnOpenFire` _equipable)
                        (message `/Game/Game/BlueprintInterface/BP_GunsInterface.CommitAmmos` _equipable))))))
              (:`then_1`
                (`AbilityTask_PlayMontageAndWait.CreatePlayMontageAndWaitProxy` "None" _output 2.0
                  (:`OnCompleted`
                    (goto _label)))))))))
    (:`else`)))