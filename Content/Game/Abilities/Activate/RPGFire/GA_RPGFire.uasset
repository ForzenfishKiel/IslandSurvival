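; GA_RPGFire is the gameplay ability that fires the player's equipped gun, by its name the RPG.
; It queries the equipable through BP_GunsInterface and, when out of ammo, checks the magazine and sends a Reloading gameplay event to the PlayerState if the check passes.
; With ammo, it plays the weapon's activate montage on the arm mesh.
; The montage's notify triggers firing and ammo commit on the authority only.
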(event `self.K2_ActivateAbility`
  (bind _asbp_ismain_player (cast `/Game/Game/Character/BP_ISMainPlayer` (`self.GetAvatarActorFromActorInfo`)))
  (bind _equipable (`ISEquipmentComponent.Equipable` (`Actor.GetComponentByClass` _asbp_ismain_player "/Script/IslandSurvival.ISEquipmentComponent"))
    (:`then`
      (if (`KismetSystemLibrary.DoesImplementInterface` _equipable "/Game/Game/BlueprintInterface/BP_GunsInterface.BP_GunsInterface_C")
        (bind _ammos (message `/Game/Game/BlueprintInterface/BP_GunsInterface.GetAmmos` _equipable))
        (if (<= _ammos 0)
          (bind _havemagazine (message `/Game/Game/BlueprintInterface/BP_GunsInterface.CallCheckMagazine` _equipable))
          (if _havemagazine
            (`AbilitySystemBlueprintLibrary.SendGameplayEventToActor` (`Pawn.PlayerState` _asbp_ismain_player) (struct :`TagName` "Blueprint.State.Reloading"))
            (`self.K2_EndAbility`)
            (else
              (`self.K2_EndAbility`)))
          (else
            (`|PlayMontage` (`ISCharacter.ArmMesh` _asbp_ismain_player) (`|GetArrayItem` (`ISEquipable.EquipableActivateAnimations` _equipable))
              (:`OnCompleted`
                (`self.K2_EndAbility`))
              (:`OnNotifyBegin`
                (`self.K2_HasAuthority`
                  (:`True`
                    (message `/Game/Game/BlueprintInterface/BP_GunsInterface.OnOpenFire` _equipable)
                    (message `/Game/Game/BlueprintInterface/BP_GunsInterface.CommitAmmos` _equipable)))))))
        (else
          (`self.K2_EndAbility`))))
    (:`else`)))