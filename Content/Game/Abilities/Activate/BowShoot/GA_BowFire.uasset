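; GA_BowFire is a Gameplay Ability that fires the player's equipped bow.
; If the CanNotBowShoot tag is present, it sends that tag as an event to the PlayerState and ends.
; Otherwise, with a valid equipable, it sends the fire event, removes GE_CanBowShoot and plays an arm montage.
; The montage notify triggers authority-only firing, ammo commit and arrow removal; only montage completion ends this path.
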(event `self.K2_ActivateAbility`
  (bind _returnvalue (`self.GetAbilitySystemComponentFromActorInfo`))
  (bind _asbp_ismain_player (cast `/Game/Game/Character/BP_ISMainPlayer` (`self.GetAvatarActorFromActorInfo`)))
  (bind _output_get (set `self.As BP ISMain Player` _asbp_ismain_player))
  (if (`GameplayTagAssetInterface.HasMatchingGameplayTag` (`self.GetAbilitySystemComponentFromActorInfo`) (struct :`TagName` "Blueprint.State.CanNotBowShoot"))
    (`AbilitySystemBlueprintLibrary.SendGameplayEventToActor` (`Pawn.PlayerState` (`self.As BP ISMain Player`)) (struct :`TagName` "Blueprint.State.CanNotBowShoot"))
    (`self.K2_EndAbility`)
    (else
      (bind _equipable (`ISEquipmentComponent.Equipable` (`Actor.GetComponentByClass` _asbp_ismain_player "/Script/IslandSurvival.ISEquipmentComponent"))
        (:`then`
          (bind _output_get_2 (set `self.Equipable` _equipable))
          (`AbilitySystemBlueprintLibrary.SendGameplayEventToActor` (`Pawn.PlayerState` _output_get) (struct :`TagName` "Input.Attack.Fire"))
          (`AbilitySystemComponent.RemoveActiveGameplayEffectBySourceEffect` _returnvalue "/Game/Game/Abilities/Activate/BowShoot/GE_CanBowShoot.GE_CanBowShoot_C" _returnvalue -1)
          (`|PlayMontage` (`ISCharacter.ArmMesh` (`self.As BP ISMain Player`)) (`|GetArrayItem` (`ISEquipable.EquipableActivateAnimations` _output_get_2) 1)
            (:`OnCompleted`
              (`self.K2_EndAbility`))
            (:`OnNotifyBegin`
              (`self.K2_HasAuthority`
                (:`True`
                  (message `/Game/Game/BlueprintInterface/BP_GunsInterface.OnOpenFire` (`self.Equipable`))
                  (message `/Game/Game/BlueprintInterface/BP_GunsInterface.CommitAmmos` (`self.Equipable`))
                  (message `/Game/Game/BlueprintInterface/BP_BowInterface.RemoveArrow` (`self.Equipable`)))))))
        (:`else`)))))