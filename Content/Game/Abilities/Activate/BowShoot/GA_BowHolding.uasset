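; Gameplay ability that draws and holds the player's equipped bow.
; Activation passes magazine and ammo checks through equipable interface messages, then plays montages on the bow's skeletal mesh and the player's arm mesh.
; On authority it adds an arrow and, when ammo runs out, discards one magazine item from the hotbar inventory and refills ammo.
; Montage blend-out or interruption ends the ability, while event-based activation stops both montages and ends it.
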(event `self.K2_ActivateAbility`
  (bind _equipable (`self.Equipable`))
  (bind _asbp_ismain_player (cast `/Game/Game/Character/BP_ISMainPlayer` (`self.GetAvatarActorFromActorInfo`)))
  (set `self.As BP ISMain Player` _asbp_ismain_player)
  (bind _equipable_2 (`ISEquipmentComponent.Equipable` (`Actor.GetComponentByClass` _asbp_ismain_player "/Script/IslandSurvival.ISEquipmentComponent"))
    (:`then`
      (bind _output_get (set `self.Equipable` _equipable_2))
      (bind _havemagazine (message `/Game/Game/BlueprintInterface/BP_GunsInterface.CallCheckMagazine` _output_get))
      (if _havemagazine
        (`|ExecutionSequence` :!label _label
          (:`then_1`
            (bind _returnskull (message `/Game/Game/BlueprintInterface/BP_GunsInterface.GetGunSkull` (`self.Equipable`)))
            (`|PlayMontage` _returnskull "/Game/Game/Items/Equiable/Bow/Texture/AM_BowAnim.AM_BowAnim"
              (:`then`
                (`self.K2_HasAuthority`
                  (:`True`
                    (bind _returnskull_2 (message `/Game/Game/BlueprintInterface/BP_GunsInterface.GetGunSkull` _equipable))
                    (message `/Game/Game/BlueprintInterface/BP_BowInterface.AddArrow` _equipable _returnskull_2)
                    (bind _ammos (message `/Game/Game/BlueprintInterface/BP_GunsInterface.GetAmmos` (`self.Equipable`)))
                    (if (<= _ammos 0)
                      (bind _outindex (message `/Game/Game/BlueprintInterface/BP_GunsInterface.GetMagazineIndex` (`self.Equipable`)))
                      (`ISItemsContainer.DiscardItem` (`Actor.GetComponentByClass` (`self.As BP ISMain Player`) "/Script/IslandSurvival.ISHotBarInventory") _outindex 1)
                      (message `/Game/Game/BlueprintInterface/BP_GunsInterface.FullAmmo` (`self.Equipable`))))))
              (:`OnBlendOut`
                (`self.K2_EndAbility` :!label _label_2))
              (:`OnInterrupted`
                (goto _label_2))))
          (:`then_2`
            (bind _output_get_2 (set `self.Arm Mesh` (`ISCharacter.ArmMesh` (`self.As BP ISMain Player`))))
            (`|PlayMontage` _output_get_2 (`|GetArrayItem` (`ISEquipable.EquipableActivateAnimations` _equipable_2)) 0.5 0.0 "Default"
              (:`OnBlendOut`
                (goto _label_2))
              (:`OnInterrupted`
                (goto _label_2)))))
        (else
          (bind _ammos_2 (message `/Game/Game/BlueprintInterface/BP_GunsInterface.GetAmmos` (`self.Equipable`)))
          (if (<= _ammos_2 0)
            (`self.K2_EndAbility`)
            (else
              (goto _label))))))
    (:`else`)))

(event `self.K2_ActivateAbilityFromEvent`
  (params (EventData :type "GameplayEventData Structure (by ref)"))
  (bind _asbp_ismain_player (cast `/Game/Game/Character/BP_ISMainPlayer` (`self.GetAvatarActorFromActorInfo`)))
  (bind _equipable (`ISEquipmentComponent.Equipable` (`Actor.GetComponentByClass` _asbp_ismain_player "/Script/IslandSurvival.ISEquipmentComponent"))
    (:`then`
      (bind _armmesh (`ISCharacter.ArmMesh` _asbp_ismain_player)
        (:`then`
          (`|ExecutionSequence`
            (:`then_0`
              (`AnimInstance.Montage_Stop` (`SkeletalMeshComponent.GetAnimInstance` _armmesh) 0.01 (`|GetArrayItem` (`ISEquipable.EquipableActivateAnimations` _equipable))))
            (:`then_1`
              (bind _returnskull (message `/Game/Game/BlueprintInterface/BP_GunsInterface.GetGunSkull` _equipable))
              (`AnimInstance.Montage_Stop` (`SkeletalMeshComponent.GetAnimInstance` _returnskull) 0.0 "/Game/Game/Items/Equiable/Bow/Texture/AM_BowAnim.AM_BowAnim")))
          (`self.K2_EndAbility`))
        (:`else`)))
    (:`else`)))