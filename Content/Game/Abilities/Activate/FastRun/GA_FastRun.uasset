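; Gameplay ability that makes the main player character run fast while a cost effect is active.
; On activation it ends immediately if the character has no horizontal velocity or CheckIsFastRun returns true.
; Otherwise it applies GE_FastRunCost, raises CharacterSpeed and waits on DetectSpeedChange.
; When that reports a speed change, it lowers the speed, removes the effect by its saved handle and ends.
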(event `self.K2_ActivateAbility`
  (bind _as_bp_ismain_player (`self.As BP ISMain Player`))
  (bind _asbp_ismain_player (cast `/Game/Game/Character/BP_ISMainPlayer` (`self.GetAvatarActorFromActorInfo`)))
  (bind _output_get (set `self.As BP ISMain Player` _asbp_ismain_player))
  (if (== (`KismetMathLibrary.VSizeXY` (`MovementComponent.Velocity` (`Character.CharacterMovement` _output_get))) 0.0)
    (`self.K2_EndAbility`)
    (else
      (bind _returnvalue (`ISCharacter.CheckIsFastRun` _output_get))
      (if _returnvalue
        (`self.K2_EndAbility`)
        (else
          (bind _returnvalue_2 (`self.BP_ApplyGameplayEffectToOwner` "/Game/Game/Abilities/Activate/FastRun/GE_FastRunCost.GE_FastRunCost_C"))
          (set `ISCharacter.CharacterSpeed` 600.0 _as_bp_ismain_player)
          (`WaitCharacterSpeedChangeToZero.DetectSpeedChange`
            (:`OnSpeedChange`
              (set `ISCharacter.CharacterSpeed` 400.0 _as_bp_ismain_player)
              (`self.BP_RemoveGameplayEffectFromOwnerWithHandle` _returnvalue_2)
              (`self.K2_EndAbility`))))))))