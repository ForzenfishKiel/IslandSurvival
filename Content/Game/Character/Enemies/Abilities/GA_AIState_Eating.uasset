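; Gameplay ability that plays an enemy's eating animation for the AI.State.Eating state.
; On activation it commits, asks the avatar for the montage mapped to that tag, and plays it.
; It ends when the montage completes, blends out, is interrupted or cancelled, or at once if none is found.
; On end, it notifies the BP_ISEnemyBase avatar that the ability has ended.
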(event `self.K2_ActivateAbility`
  (`self.K2_CommitAbility`)
  (bind _returnvalue (message `ISCombatInterface.FindMontageFromTag` (`self.GetAvatarActorFromActorInfo`) (struct :`TagName` "AI.State.Eating")))
  (`/Engine/EditorBlueprintResources/StandardMacros.IsValid` (break `TaggedMontage` _returnvalue)
    (:`Is Valid`
      (`AbilityTask_PlayMontageAndWait.CreatePlayMontageAndWaitProxy` "None" (break `TaggedMontage` _returnvalue)
        (:`OnCompleted`
          _)
        (:`OnBlendOut`
          _)
        (:`OnInterrupted`
          _)
        (:`OnCancelled`
          _))
      (`self.K2_EndAbility`))
    (:`Is Not Valid`
      (`self.K2_EndAbility`))))

(event `self.K2_OnEndAbility`
  (params (bWasCancelled :type Boolean))
  (bind _asbp_isenemy_base (cast `/Game/Game/Character/Enemies/BP_ISEnemyBase` (`self.GetAvatarActorFromActorInfo`)))
  (`/Game/Game/Character/Enemies/BP_ISEnemyBase.Call Ability End` _asbp_isenemy_base))