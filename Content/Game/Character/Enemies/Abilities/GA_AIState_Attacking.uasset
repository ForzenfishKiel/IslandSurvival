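; Gameplay ability for an enemy's attacking AI state that plays an attack montage and deals melee damage to players.
; It fetches the montage by the AI.State.Attacking tag, then waits for a gameplay event with that tag.
; On authority, a short forward box trace from the eyes damages a pawn implementing ISPlayerInterface, with debug drawing left on.
; Ending the ability notifies BP_ISEnemyBase through CallCallAbilityEnd.
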(event `self.K2_ActivateAbility`
  (bind _returnvalue (`self.GetAvatarActorFromActorInfo`))
  (bind (_outlocation _outrotation) (`Actor.GetActorEyesViewPoint` _returnvalue))
  (bind _returnvalue_2 (+ _outlocation (* (`Actor.GetActorForwardVector` _returnvalue) 90.0)))
  (`self.K2_CommitAbility`)
  (bind _returnvalue_3 (message `ISCombatInterface.FindMontageFromTag` (`self.GetAvatarActorFromActorInfo`) (struct :`TagName` "AI.State.Attacking")))
  (`/Engine/EditorBlueprintResources/StandardMacros.IsValid` (break `TaggedMontage` _returnvalue_3)
    (:`Is Valid`
      (`AbilityTask_PlayMontageAndWait.CreatePlayMontageAndWaitProxy` "None" (break `TaggedMontage` _returnvalue_3)
        (:`then`
          (`AbilityAsync_WaitGameplayEvent.WaitGameplayEventToActor` (`self.GetAvatarActorFromActorInfo`) (struct :`TagName` "AI.State.Attacking") true
            (:`EventReceived`
              (`self.K2_HasAuthority`
                (:`True`
                  (`KismetSystemLibrary.DrawDebugSphere` _outlocation 100.0 12 (struct :`G` 1.0 :`B` 0.257701 :`A` 1.0) 5.0)
                  (`KismetSystemLibrary.DrawDebugSphere` _returnvalue_2 100.0 12 (struct :`G` 1.0 :`B` 0.28806 :`A` 1.0) 5.0)
                  (bind (_outhit _returnvalue_4) (`KismetSystemLibrary.BoxTraceSingleForObjects` _outlocation _returnvalue_2 (0.0 0.0 0.0) _outrotation (`|MakeArray` "ObjectTypeQuery3" :!type "EObjectTypeQuery Enum") false (`|MakeArray` _returnvalue) "ForDuration"))
                  (if _returnvalue_4
                    (if (`KismetSystemLibrary.DoesImplementInterface` (`.HitActor` (`GameplayStatics.BreakHitResult` _outhit)) "/Script/IslandSurvival.ISPlayerInterface")
                      (message `ISCombatInterface.ApplyDamageToTarget` (`self.GetAvatarActorFromActorInfo`) (`.HitActor` (`GameplayStatics.BreakHitResult` _outhit)))
                      (`self.K2_EndAbility`)
                      (else
                        (`self.K2_EndAbility`)))
                    (else
                      (`self.K2_EndAbility`))))))))
        (:`OnCompleted`
          (`self.K2_EndAbility` :!label _label))
        (:`OnBlendOut`
          (goto _label))
        (:`OnInterrupted`
          (goto _label))
        (:`OnCancelled`
          (goto _label))))))

(event `self.K2_OnEndAbility`
  (params (bWasCancelled :type Boolean))
  (bind _asbp_isenemy_base (cast `/Game/Game/Character/Enemies/BP_ISEnemyBase` (`self.GetAvatarActorFromActorInfo`)))
  (`/Game/Game/Character/Enemies/BP_ISEnemyBase.Call Ability End` _asbp_isenemy_base))