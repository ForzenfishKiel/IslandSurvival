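; Gameplay ability for the wolf enemy's AI attacking state, playing an attack montage and dealing melee damage.
; The avatar supplies the montage by tag, and a one-shot gameplay event triggers an authority-only box trace forward from the WOLFHAND socket, with debug drawing enabled.
; A hit pawn implementing the player interface takes damage through an avatar message.
; The ability ends after the trace or montage, then notifies BP_ISEnemyBase.
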(event `self.K2_ActivateAbility`
  (bind _returnvalue (`self.GetAvatarActorFromActorInfo`))
  (`self.K2_CommitAbility`)
  (bind _returnvalue_2 (message `ISCombatInterface.FindMontageFromTag` (`self.GetAvatarActorFromActorInfo`) (struct :`TagName` "AI.State.Attacking")))
  (`/Engine/EditorBlueprintResources/StandardMacros.IsValid` (break `TaggedMontage` _returnvalue_2)
    (:`Is Valid`
      (`AbilityTask_PlayMontageAndWait.CreatePlayMontageAndWaitProxy` "None" (break `TaggedMontage` _returnvalue_2)
        (:`then`
          (`AbilityAsync_WaitGameplayEvent.WaitGameplayEventToActor` (`self.GetAvatarActorFromActorInfo`) (struct :`TagName` "AI.State.Attacking") true
            (:`EventReceived`
              (`self.K2_HasAuthority`
                (:`True`
                  (bind _returnvalue_3 (message `ISCombatInterface.GetTargetSkeletalMeshComponent` _returnvalue))
                  (bind _returnvalue_4 (`SceneComponent.GetSocketLocation` _returnvalue_3 "WOLFHAND"))
                  (bind (_outhit _returnvalue_5) (`KismetSystemLibrary.BoxTraceSingleForObjects` _returnvalue_4 (+ _returnvalue_4 (* (`Actor.GetActorForwardVector` _returnvalue) 40.0)) (0.0 0.0 0.0) (struct) (`|MakeArray` "ObjectTypeQuery3" :!type "EObjectTypeQuery Enum") false (`|MakeArray` _returnvalue) "ForDuration"))
                  (if _returnvalue_5
                    (if (`KismetSystemLibrary.DoesImplementInterface` (`.HitActor` (`GameplayStatics.BreakHitResult` _outhit)) "/Script/IslandSurvival.ISPlayerInterface")
                      (message `ISCombatInterface.ApplyDamageToTarget` (`self.GetAvatarActorFromActorInfo`) (`.HitActor` (`GameplayStatics.BreakHitResult` _outhit)))
                      (`self.K2_EndAbility`)
                      (else
                        (`self.K2_EndAbility`)))
                    (else
                      (`self.K2_EndAbility`))))))))
        (:`OnCompleted`
          (`self.K2_EndAbility` :!label _label))
        (:`OnBlendOut`
          (goto _label))
        (:`OnInterrupted`
          (goto _label))
        (:`OnCancelled`
          (goto _label))))))

(event `self.K2_OnEndAbility`
  (params (bWasCancelled :type Boolean))
  (bind _asbp_isenemy_base (cast `/Game/Game/Character/Enemies/BP_ISEnemyBase` (`self.GetAvatarActorFromActorInfo`)))
  (`/Game/Game/Character/Enemies/BP_ISEnemyBase.Call Ability End` _asbp_isenemy_base))