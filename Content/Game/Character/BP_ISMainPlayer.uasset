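; Main player character Blueprint handling equipment, resource collection and building placement feedback.
; Equipment component events drive equip and unequip along with their client-side calls; hotbar inventory events only print debug text.
; CollectAction box-traces ahead of the camera via CollectActionOnSever, sending collection messages to new Tropical targets, cached until EndCollectOnSever clears them.
; Building component callback tints the preview green or red from overlap, foundation and floating checks, setting CanBeBuild.
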(event `self.ReceiveBeginPlay`)

(event `self.ReceiveTick`
  (params (DeltaSeconds :type "Float (single-precision)")))

(event `self.CharacterEquipment.OnEquip`
  (params (TargetItemInfo :type "ItemInformation Structure"))
  ;[0 0.246 1] 设置角色装备
  (`ISEquipmentComponent.Equip` (`self.CharacterEquipment`) TargetItemInfo)
  (`ISEquipmentComponent.SpawnEquipOnClient` (`self.CharacterEquipment`) TargetItemInfo))

(event `self.CharacterEquipment.OnUnEquip`
  ;[0 0.246 1] 设置角色装备
  (`ISEquipmentComponent.UnEquip` (`self.CharacterEquipment`))
  (`ISEquipmentComponent.UnEquipOnClient` (`self.CharacterEquipment`)))

(event `self.CharacterHotBarInventory.ItemPickup`
  (params (TargetItemInfo :type "ItemInformation Structure"))
  ;[0 0.246 1] 设置角色装备
  (`KismetSystemLibrary.PrintString` "Pick Up"))

(event `self.CharacterHotBarInventory.InventoryUpdate`
  ;[0 0.246 1] 设置角色装备
  (`KismetSystemLibrary.PrintString` "Inventory Update"))

(event `CollectAction`
  ;[0.9845 0.2634 1] 人物采集
  (bind (_start _end _returnrotaiton) (`self.GetActorForwardLocation` 45.0 150.0)
    (:`OutPut`
      (`self.CollectActionOnSever` _start _end _returnrotaiton))))

(event `CollectActionOnSever`
  (params (Start :type "Vector Structure") (End :type "Vector Structure") (Rotation :type "Rotator Structure"))
  ;[0.9845 0.2634 1] 人物采集
  (bind _outhits (`KismetSystemLibrary.BoxTraceMultiForObjects` Start End (1.0 1.0 1.0) Rotation (`|MakeArray` "ObjectTypeQuery7" :!type "EObjectTypeQuery Enum") false (`|MakeArray` self :!type "Actor Object Reference") "None" true (struct :`G` 0.78404 :`B` 1.0 :`A` 1.0) (struct :`G` 1.0 :`A` 1.0) 1.0))
  (for _array_element _outhits
    (`self.TryToPickUp` (`.HitActor` (`GameplayStatics.BreakHitResult` _array_element)))))

(event `EndCollectOnSever`
  ;[0.9845 0.2634 1] 人物采集
  (`|ExecutionSequence`
    (:`then_0`
      (`self.Array Element Hit Actor`
        (:`then`
          (set `self.Array Element Hit Actor` null))
        (:`else`)))
    (:`then_1`
      (set `ISInteractionComponent.LastActor` null (`self.ISInteractionComponent`))
      (set `ISInteractionComponent.LastComponent` null (`self.ISInteractionComponent`)))))

(event `self.ISBuildingComponent.OnCallSetMaterial`
  (params (BuildBooleanCheck :type "ISBuildBooleanCheck Structure"))
  ;[1 0.6587 0.1146] 设置预览建筑物颜色
  (if BuildBooleanCheck_bCanBeBuildOnFoundation
    (if BuildBooleanCheck_bCheckBuildFoundation
      (if (not BuildBooleanCheck_bIsOverlap) :!label _label
        (`PrimitiveComponent.SetMaterial` BuildBooleanCheck_BuildMesh BuildBooleanCheck_TargetIndex "/Game/Game/BuildingSystem/Materials/M_Green.M_Green" :!label _label_2)
        (set `ISBuildingComponent.bCanBeBuild` true (`self.ISBuildingComponent`))
        (else
          (`PrimitiveComponent.SetMaterial` BuildBooleanCheck_BuildMesh BuildBooleanCheck_TargetIndex "/Game/Game/BuildingSystem/Materials/M_Red.M_Red" :!label _label_3)
          (set `ISBuildingComponent.bCanBeBuild` false (`self.ISBuildingComponent`))))
      (else
        (goto _label_3)))
    (elif BuildBooleanCheck_bDoFloatCheck
      (if (and (not BuildBooleanCheck_bIsOverlap) BuildBooleanCheck_bIsFloating)
        (goto _label_2)
        (else
          (goto _label_3)))
      (else
        (goto _label)))))

(fn `TryToPickUp`
  (params (InActor :type "Actor Object Reference"))
  (if (== InActor (`self.Array Element Hit Actor`))
    (return)
    (else
      (bind _output_get (set `self.Array Element Hit Actor` InActor))
      (bind _returnvalue (message `ISCollectibleInterface.GetTargetClass` _output_get))
      (switch `ECollectibleClass` _returnvalue
        (:`Tropical`
          (bind _array_element_hit_actor (`self.Array Element Hit Actor`)
            (:`then`
              (message `ISCollectibleInterface.CollectionExecution` _array_element_hit_actor self self))
            (:`else`)))))))

(fn `UserConstructionScript`)