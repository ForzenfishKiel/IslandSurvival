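; BP_EquipableBase is a base Blueprint for equipable items, with gun-style queries for child classes to override.
; Magazine check, ammo, max ammo, magazine index and gun skull functions are stubs returning empty or default values.
; GetCharacterArrowLoc casts the owner to BP_ISMainPlayer and projects start and end points from its eye location along camera forward, also returning view rotation.
; Its event graph and construction script are empty.
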(fn `CallCheckMagazine`
  (returns (HaveMagazine :type Boolean))
  (return false))

(fn `Get MaxAmmo`
  (returns (OutMaxAmmo :type Integer))
  (return 0))

(fn `GetAmmos`
  (returns (Ammos :type Integer))
  (return 0))

(fn `GetGunSkull`
  (returns (ReturnSkull :type "SkeletalMeshComponent Object Reference"))
  (return null))

(fn `GetMagazineIndex`
  (returns (OutIndex :type Integer))
  (return 0))

(fn `UserConstructionScript`)