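; BP_Rifle is a rifle weapon item that fires BP_Ammo projectiles and tracks its own ammo count.
; On open fire it takes the owning BP_ISMainPlayer's camera view and passes it to SpawnAmmoOnServer, which spawns the projectile with a limited lifespan to avoid bullet buildup.
; Separate events play a scaled-down explosion emitter at the mesh's Muzzle socket and decrement the ammo count, which GetAmmos exposes.
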(event `self.ReceiveBeginPlay`
  (`parent.ReceiveBeginPlay`))

(event `/Game/Game/BlueprintInterface/BP_GunsInterface.PlayMuzzle`
  (bind _skeletalmesh (`self.SkeletalMesh`))
  (`GameplayStatics.SpawnEmitterAtLocation` "/Game/StarterContent/Particles/P_Explosion.P_Explosion" (`SceneComponent.GetSocketLocation` _skeletalmesh "Muzzle") (`SceneComponent.GetSocketRotation` _skeletalmesh "Muzzle") (0.1 0.1 0.1)))

(event `/Game/Game/BlueprintInterface/BP_GunsInterface.OnOpenFire`
  (bind _asbp_ismain_player (cast `/Game/Game/Character/BP_ISMainPlayer` (`self.GetOwner`)))
  (bind _desiredview (`CameraComponent.GetCameraView` (`ISCharacter.CameraComponent` _asbp_ismain_player) 0.0))
  (`self.SpawnAmmoOnServer` (`KismetMathLibrary.MakeTransform` (break `MinimalViewInfo` _desiredview) (`.Rotation` (break `MinimalViewInfo` _desiredview)))))

(event `SpawnAmmoOnServer`
  (params (TargetPoint :type "Transform Structure"))
  (bind _returnvalue (`|SpawnActorFromClass` "/Game/Game/Items/Equiable/Guns/Ammos/BP_Ammo.BP_Ammo_C" TargetPoint "Undefined" "MultiplyWithRoot" null null))
  (`self.SetLifeSpan` _returnvalue 10.0) ; 防止产生过多子弹
)

(event `/Game/Game/BlueprintInterface/BP_GunsInterface.CommitAmmos`
  (`/Engine/EditorBlueprintResources/StandardMacros.DecrementInt` (`self.Ammos`)))

(fn `GetAmmos`
  (returns (Ammos :type Integer))
  (return (`self.Ammos`)))

(fn `UserConstructionScript`
  (`parent.UserConstructionScript`))