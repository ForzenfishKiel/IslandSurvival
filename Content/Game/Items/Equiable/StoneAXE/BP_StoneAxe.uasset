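; BP_StoneAxe is an equipable stone axe that harvests trees and damages buildings.
; On activation it computes a short segment along the owning player's camera forward, then passes it to ActivateAbilityOnServer for a multi-object box trace with debug drawing.
; Tree hits receive a collection message, and ISBuildInterface actors receive a build-breaking message.
; The last hit actor is cached to stop repeat hits and cleared when the ability ends.
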(event `ISItemInterface.EquipableAbilityActivate`
  ;[0.3803 0 1] 采集执行
  (`self.GetRotationVector`))

(event `GetRotationVector`
  ;[0.3803 0 1] 采集执行
  (bind (_returnstart _returnend _returnrotation) (`self.GetCharacterArrowLoc` 45.0 80.0))
  (`self.ActivateAbilityOnServer` _returnstart _returnend _returnrotation))

(event `ActivateAbilityOnServer`
  (params (InTargetStart :type "Vector Structure") (InTargetEnd :type "Vector Structure") (InTargetRotaion :type "Rotator Structure"))
  ;[0.3803 0 1] 采集执行
  (bind _outhits (`KismetSystemLibrary.BoxTraceMultiForObjects` InTargetStart InTargetEnd (1.0 1.0 1.0) InTargetRotaion (`|MakeArray` "ObjectTypeQuery7" "ObjectTypeQuery6" :!type "EObjectTypeQuery Enum") false (`|MakeArray` (`self.GetOwner`)) "ForDuration" true (struct :`R` 1.0 :`A` 1.0) (struct :`G` 1.0 :`A` 1.0) 1.0))
  (for _array_element _outhits
    (if (== (`.HitActor` (`GameplayStatics.BreakHitResult` _array_element)) (`self.Array Element Hit Actor`))
      (break)
      (else
        (set `self.Array Element Hit Actor` (`.HitActor` (`GameplayStatics.BreakHitResult` _array_element)))
        (`self.TryToPickUp` (`.HitActor` (`GameplayStatics.BreakHitResult` _array_element)))
        (`self.TryToBrakeBuilding` (`.HitActor` (`GameplayStatics.BreakHitResult` _array_element)))))))

(event `ISEquipableInterface.EndAbilityActivate`
  ;[0.3803 0 1] 采集执行
  (`self.Array Element Hit Actor`
    (:`then`
      (set `self.Array Element Hit Actor` null))
    (:`else`)))

(fn `TryToBrakeBuilding`
  (params (InActor :type "Actor Object Reference"))
  (if (`KismetSystemLibrary.DoesImplementInterface` InActor "/Script/IslandSurvival.ISBuildInterface")
    (message `ISBuildInterface.OnBuildBroking` InActor (`self.GetOwner`))
    (return)))

(fn `TryToPickUp`
  (params (InActor :type "Actor Object Reference"))
  (bind _returnvalue (message `ISCollectibleInterface.GetTargetClass` InActor))
  (switch `ECollectibleClass` _returnvalue
    (:`Tree`
      (bind _array_element_hit_actor (`self.Array Element Hit Actor`)
        (:`then`
          (message `ISCollectibleInterface.CollectionExecution` _array_element_hit_actor (`self.GetOwner`) self)
          (return))
        (:`else`)))))

(fn `UserConstructionScript`)