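; Iron axe equipable that, on activation, box-traces ahead of the player's camera through a server-named event for harvesting, building breaking and damage.
; Instanced mesh hits look up a harvest asset and swap the instance for an actor, which goes to the Tree/Corpse collection and build-interface checks.
; Other hits run the same helpers and send damage, caching the actor to skip repeat hits until the ability ends.
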(event `ISItemInterface.EquipableAbilityActivate`
  ;[0.3803 0 1] 采集执行
  (`self.GetRotationVector`))

(event `GetRotationVector`
  ;[0.3803 0 1] 采集执行
  (bind (_returnstart _returnend _returnrotation) (`self.GetCharacterArrowLoc` 45.0 80.0))
  (`self.ActivateAbilityOnServer` _returnstart _returnend _returnrotation))

(event `ActivateAbilityOnServer`
  (params (InTargetStart :type "Vector Structure") (InTargetEnd :type "Vector Structure") (InTargetRotaion :type "Rotator Structure"))
  ;[0.3803 0 1] 采集执行
  (bind _outhit (`KismetSystemLibrary.BoxTraceSingleForObjects` InTargetStart InTargetEnd (0.0 0.0 0.0) InTargetRotaion (`|MakeArray` "ObjectTypeQuery7" "ObjectTypeQuery6" "ObjectTypeQuery3" :!type "EObjectTypeQuery Enum") false (`|MakeArray` (`self.GetOwner`))))
  (`/Engine/EditorBlueprintResources/StandardMacros.IsValid` (`.HitComponent` (`GameplayStatics.BreakHitResult` _outhit))
    (:`Is Valid`
      (bind _asinstanced_static_mesh_component (cast `InstancedStaticMeshComponent` (`.HitComponent` (`GameplayStatics.BreakHitResult` _outhit)))
        (:`then`
          (bind _returnvalue (`self.CheckHarvestDataAsset` (`KismetSystemLibrary.GetObjectName` _asinstanced_static_mesh_component)))
          (bind _returnvalue_2 (`self.ReplaceToActor` _returnvalue _asinstanced_static_mesh_component (`.HitItem` (`GameplayStatics.BreakHitResult` _outhit))))
          (`self.TryToPickUp` _returnvalue_2)
          (`self.TryToBrakeBuilding` _returnvalue_2))
        (:`CastFailed`
          (if (not (== (`.HitActor` (`GameplayStatics.BreakHitResult` _outhit)) (`self.Array Element Hit Actor`)))
            (set `self.Array Element Hit Actor` (`.HitActor` (`GameplayStatics.BreakHitResult` _outhit)))
            (`self.TryToPickUp` null)
            (`self.TryToBrakeBuilding` null)
            (message `ISCombatInterface.ApplyDamageToTarget` (`self.GetOwner`) (`self.Array Element Hit Actor`))))))))

(event `ISEquipableInterface.EndAbilityActivate`
  ;[0.3803 0 1] 采集执行
  (`self.Array Element Hit Actor`
    (:`then`
      (set `self.Array Element Hit Actor` null))
    (:`else`)))

(fn `TryToBrakeBuilding`
  (params (InActor :type "Actor Object Reference"))
  (if (`KismetSystemLibrary.DoesImplementInterface` InActor "/Script/IslandSurvival.ISBuildInterface")
    (message `ISBuildInterface.OnBuildBroking` InActor (`self.GetOwner`))
    (return)))

(fn `TryToPickUp`
  (params (InActor :type "Actor Object Reference"))
  (bind _returnvalue (message `ISCollectibleInterface.GetTargetClass` InActor))
  (switch `ECollectibleClass` _returnvalue
    (:`Tree`
      _)
    (:`Corpse`
      _))
  (bind _array_element_hit_actor (`self.Array Element Hit Actor`)
    (:`then`
      (message `ISCollectibleInterface.CollectionExecution` _array_element_hit_actor (`self.GetOwner`) self)
      (return))
    (:`else`)))

(fn `UserConstructionScript`)