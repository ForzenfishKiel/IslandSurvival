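; BP_RPG is an equippable RPG launcher that fires rocket actors for its owning player.
; On fire, it takes the owner's camera view and passes it to SpawnAmmoOnServer, which spawns a short-lived BP_RPGAmmo owned by that player.
; Separate events play the muzzle emitter at the Muzzle socket, decrement ammo and refill it to the maximum through a server-named event.
; Getter functions expose ammo counts and magazine lookups by MagazineID.
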(event `/Game/Game/BlueprintInterface/BP_GunsInterface.PlayMuzzle`
  (`GameplayStatics.SpawnEmitterAtLocation` "/Game/WuContent/Weapon/RPG7/FX/RPGFire.RPGFire" (`SceneComponent.GetSocketLocation` (`self.SkeletalMesh`) "Muzzle")))

(event `/Game/Game/BlueprintInterface/BP_GunsInterface.OnOpenFire`
  (bind _asbp_ismain_player (cast `/Game/Game/Character/BP_ISMainPlayer` (`self.GetOwner`)))
  (bind _desiredview (`CameraComponent.GetCameraView` (`ISCharacter.CameraComponent` _asbp_ismain_player) 0.0))
  (`self.SpawnAmmoOnServer` (`KismetMathLibrary.MakeTransform` (break `MinimalViewInfo` _desiredview) (`.Rotation` (break `MinimalViewInfo` _desiredview)))))

(event `SpawnAmmoOnServer`
  (params (InTransfrom :type "Transform Structure"))
  (bind _returnvalue (`|SpawnActorFromClass` "/Game/Game/Items/Equiable/RPG/BP_RPGAmmo.BP_RPGAmmo_C" InTransfrom "Undefined" "MultiplyWithRoot" (`self.GetOwner`) null))
  (`self.SetLifeSpan` _returnvalue 5.0))

(event `/Game/Game/BlueprintInterface/BP_GunsInterface.CommitAmmos`
  (`/Engine/EditorBlueprintResources/StandardMacros.DecrementInt` (`self.Ammos`)))

(event `/Game/Game/BlueprintInterface/BP_GunsInterface.FullAmmo`
  (`self.FuulAmmoOnServer`))

(event `FuulAmmoOnServer`
  (set `self.Ammos` (`KismetMathLibrary.Clamp` (+ (`self.Ammos`) (`self.MaxAmmos`)) 0 (`self.MaxAmmos`))))

(fn `CallCheckMagazine`
  (returns (HaveMagazine :type Boolean))
  (bind _returnvalue (`self.CheckMagazine` (`self.MagazineID`)))
  (bind _returnvalue_2 (!= _returnvalue -1))
  (if _returnvalue_2
    (return _returnvalue_2)))

(fn `Get MaxAmmo`
  (returns (OutMaxAmmo :type Integer))
  (return (`self.MaxAmmos`)))

(fn `GetAmmos`
  (returns (Ammos :type Integer))
  (return (`self.Ammos`)))

(fn `GetMagazineIndex`
  (returns (OutIndex :type Integer))
  (bind _returnvalue (`self.CheckMagazine` (`self.MagazineID`)))
  (bind _output_get (set `self.ReturnMagazineIndex` _returnvalue))
  (return _output_get))

(fn `UserConstructionScript`)