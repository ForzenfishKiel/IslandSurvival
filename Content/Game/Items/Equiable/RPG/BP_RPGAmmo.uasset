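; BP_RPGAmmo is the RPG round that, on overlap, applies an area blast to buildable actors.
; Its Sphere overlap prints the hit component and calls OnExplore, which runs a multi-sphere trace around the actor, ignoring the owner.
; Hit actors implementing ISBuildInterface receive OnBuildBrokingMessage with the owner, skipping only consecutive repeats via a last-hit variable.
; Debug print and trace drawing are enabled, and the round never destroys itself here.
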(event `self.Sphere.OnComponentBeginOverlap`
  (params (OverlappedComponent :type "PrimitiveComponent Object Reference") (OtherActor :type "Actor Object Reference") (OtherComp :type "PrimitiveComponent Object Reference") (OtherBodyIndex :type Integer) (bFromSweep :type Boolean) (SweepResult :type "HitResult Structure (by ref)"))
  (`KismetSystemLibrary.PrintString` (`KismetSystemLibrary.GetDisplayName` OtherComp) true true (struct :`G` 0.66 :`B` 1.0 :`A` 1.0) 20.0)
  (`/Engine/EditorBlueprintResources/StandardMacros.IsValid` OtherActor
    (:`Is Valid`
      (`self.OnExplore`))))

(event `OnExplore`
  (bind _returnvalue (`self.K2_GetActorLocation`))
  (bind (_outhits _returnvalue_2) (`KismetSystemLibrary.SphereTraceMulti` _returnvalue _returnvalue 200.0 "TraceTypeQuery1" false (`|MakeArray` (`self.GetOwner`)) "ForDuration" true (struct :`R` 1.0 :`A` 1.0) (struct :`G` 1.0 :`A` 1.0) 10.0))
  (if _returnvalue_2
    (for _array_element _outhits
      (if (`KismetSystemLibrary.DoesImplementInterface` (`.HitActor` (`GameplayStatics.BreakHitResult` _array_element)) "/Script/IslandSurvival.ISBuildInterface")
        (if (!= (`.HitActor` (`GameplayStatics.BreakHitResult` _array_element)) (`self.Array Element Hit Actor`))
          (set `self.Array Element Hit Actor` (`.HitActor` (`GameplayStatics.BreakHitResult` _array_element)))
          (message `ISBuildInterface.OnBuildBroking` (`.HitActor` (`GameplayStatics.BreakHitResult` _array_element)) (`self.GetOwner`)))))
    (set `self.Array Element Hit Actor` null)))

(fn `UserConstructionScript`)