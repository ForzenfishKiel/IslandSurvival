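; Equipable rock item that players pick up into their items container and use as a tool for collecting from trees.
; Activating it passes camera-based points to an OnServer event that box-traces for harvestable objects.
; Instanced mesh hits are swapped for actors via a harvest data lookup.
; Tree-type targets trigger a collection message on the cached hit actor, which prevents repeat hits until the ability ends.
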(event `ISEquipableInterface.OnEquipableWasInteract`
  (params (InteractingActor :type "Actor Object Reference"))
  (`self.PickUpOnServer` InteractingActor))

(event `PickUpOnServer`
  (params (InActor :type "Actor Object Reference"))
  (bind _asbp_ismain_player (cast `/Game/Game/Character/BP_ISMainPlayer` InActor))
  (`ISItemsContainer.PickUpItemForID` (`self.GetComponentByClass` _asbp_ismain_player "/Script/IslandSurvival.ISItemsContainer") _asbp_ismain_player "4" 1)
  (`self.K2_DestroyActor`))

(event `ISItemInterface.EquipableAbilityActivate`
  (bind (_returnstart _returnend _returnrotation) (`self.GetCharacterArrowLoc` 45.0 80.0))
  (`self.ActivateAbilityOnServer` _returnstart _returnend _returnrotation))

(event `ActivateAbilityOnServer`
  (params (InTargetStart :type "Vector Structure") (InTargetEnd :type "Vector Structure") (InTargetRotation :type "Rotator Structure"))
  (bind _outhit (`KismetSystemLibrary.BoxTraceSingleForObjects` InTargetStart (0.0 0.0 0.0) InTargetEnd (struct) (`|MakeArray` "ObjectTypeQuery7" "ObjectTypeQuery6" :!type "EObjectTypeQuery Enum") false (`|MakeArray` (`self.GetOwner`))))
  (`/Engine/EditorBlueprintResources/StandardMacros.IsValid` (`.HitComponent` (`GameplayStatics.BreakHitResult` _outhit))
    (:`Is Valid`
      (bind _asinstanced_static_mesh_component (cast `InstancedStaticMeshComponent` (`.HitComponent` (`GameplayStatics.BreakHitResult` _outhit)))
        (:`then`
          (bind _returnvalue (`self.CheckHarvestDataAsset` (`KismetSystemLibrary.GetObjectName` _asinstanced_static_mesh_component)))
          (bind _returnvalue_2 (`self.ReplaceToActor` _returnvalue _asinstanced_static_mesh_component (`.HitItem` (`GameplayStatics.BreakHitResult` _outhit))))
          (`self.TryToPickUp` _returnvalue_2))
        (:`CastFailed`
          (if (not (== (`.HitActor` (`GameplayStatics.BreakHitResult` _outhit)) (`self.Array Element Hit Actor`)))
            (set `self.Array Element Hit Actor` (`.HitActor` (`GameplayStatics.BreakHitResult` _outhit)))
            (`self.TryToPickUp` (`self.Array Element Hit Actor`))))))))

(event `ISEquipableInterface.EndAbilityActivate`
  (`self.Array Element Hit Actor`
    (:`then`
      (set `self.Array Element Hit Actor` null))
    (:`else`)))

(fn `TryToPickUp`
  (params (InActor :type "Actor Object Reference"))
  (bind _returnvalue (message `ISCollectibleInterface.GetTargetClass` InActor))
  (switch `ECollectibleClass` _returnvalue
    (:`Tree`
      (bind _array_element_hit_actor (`self.Array Element Hit Actor`)
        (:`then`
          (message `ISCollectibleInterface.CollectionExecution` _array_element_hit_actor (`self.GetOwner`) self)
          (return))
        (:`else`)))))

(fn `UserConstructionScript`
  (`parent.UserConstructionScript`))