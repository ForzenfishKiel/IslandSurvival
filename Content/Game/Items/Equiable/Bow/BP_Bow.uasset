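; BP_Bow is an equippable bow weapon that fires BP_Arrow actors from the owning player's view.
; Firing passes the camera transform to an OnServer event, which spawns a limited-lifespan arrow owned by the bow's owner.
; Similar OnServer events refill clamped ammo and toggle the static mesh as the arrow is added or removed.
; Helper functions find the magazine index by ArrowID and expose the skeletal mesh and ammo counts.
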(event `/Game/Game/BlueprintInterface/BP_GunsInterface.CommitAmmos`
  (`/Engine/EditorBlueprintResources/StandardMacros.DecrementInt` (`self.Ammos`)))

(event `/Game/Game/BlueprintInterface/BP_GunsInterface.FullAmmo`
  (`self.FullAmmoOnServer`))

(event `FullAmmoOnServer`
  (set `self.Ammos` (`KismetMathLibrary.Clamp` (+ (`self.Ammos`) (`self.MaxAmmos`)) 0 (`self.MaxAmmos`))))

(event `/Game/Game/BlueprintInterface/BP_BowInterface.AddArrow`
  (params (InSkull :type "SkeletalMeshComponent Object Reference"))
  (`self.AddArrowOnServer` InSkull))

(event `AddArrowOnServer`
  (params (InSkull :type "SkeletalMeshComponent Object Reference"))
  (`SceneComponent.SetVisibility` (`self.StaticMesh`) true false))

(event `/Game/Game/BlueprintInterface/BP_BowInterface.RemoveArrow`
  (`self.RemoveArrowOnServer`))

(event `RemoveArrowOnServer`
  (`SceneComponent.SetVisibility` (`self.StaticMesh`) false false))

(event `/Game/Game/BlueprintInterface/BP_GunsInterface.OnOpenFire`
  (bind _asbp_ismain_player (cast `/Game/Game/Character/BP_ISMainPlayer` (`self.GetOwner`)))
  (bind _desiredview (`CameraComponent.GetCameraView` (`ISCharacter.CameraComponent` _asbp_ismain_player) 0.0))
  (`self.OnBowOpenFireOnServer` (`KismetMathLibrary.MakeTransform` (break `MinimalViewInfo` _desiredview) (`.Rotation` (break `MinimalViewInfo` _desiredview)))))

(event `OnBowOpenFireOnServer`
  (params (InTransForm :type "Transform Structure"))
  (bind _returnvalue (`|SpawnActorFromClass` "/Game/Game/Items/Equiable/Bow/BP_Arrow.BP_Arrow_C" InTransForm "AlwaysSpawn" "MultiplyWithRoot" (`self.GetOwner`) null))
  (`self.SetLifeSpan` _returnvalue 60.0))

(fn `CallCheckMagazine`
  (returns (HaveMagazine :type Boolean))
  (bind _returnvalue (`self.CheckMagazine` (`self.ArrowID`)))
  (bind _returnvalue_2 (!= _returnvalue -1))
  (if _returnvalue_2
    (set `self.ArrowIndex` _returnvalue)
    (return _returnvalue_2)))

(fn `Get MaxAmmo`
  (returns (OutMaxAmmo :type Integer))
  (return (`self.MaxAmmos`)))

(fn `GetAmmos`
  (returns (Ammos :type Integer))
  (return (`self.Ammos`)))

(fn `GetGunSkull`
  (returns (ReturnSkull :type "SkeletalMeshComponent Object Reference"))
  (return (`self.SkeletalMesh`)))

(fn `GetMagazineIndex`
  (returns (OutIndex :type Integer))
  (bind _returnvalue (`self.CheckMagazine` (`self.ArrowID`)))
  (if (!= _returnvalue -1)
    (return _returnvalue)))

(fn `UserConstructionScript`
  (`parent.UserConstructionScript`))