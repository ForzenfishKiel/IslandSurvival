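; Equipable stone spear that strikes what is in front of the player and harvests corpses.
; On activation it builds a short segment along the camera's forward vector and passes it to ActivateAbilityOnServer for a debug-drawn multi box trace.
; Hits trigger collection on Corpse collectibles and a damage message through the owner.
; The last hit actor is cached to break the loop on a repeat, then cleared when the ability ends.
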(event `ISItemInterface.EquipableAbilityActivate`
  (`self.GetCharacterLocandRot`))

(event `GetCharacterLocandRot`
  (bind (_returnstart _returnend _returnrotation) (`self.GetCharacterArrowLoc` 100.0 140.0))
  (`self.ActivateAbilityOnServer` _returnstart _returnend _returnrotation))

(event `ActivateAbilityOnServer`
  (params (InTargetStart :type "Vector Structure") (InTargetEnd :type "Vector Structure") (InTargetRotation :type "Rotator Structure"))
  (bind _outhits (`KismetSystemLibrary.BoxTraceMultiForObjects` InTargetStart InTargetEnd (0.0 0.0 0.0) InTargetRotation (`|MakeArray` "ObjectTypeQuery3" "ObjectTypeQuery7" :!type "EObjectTypeQuery Enum") false (`|MakeArray` (`self.GetOwner`)) "ForDuration"))
  (for _array_element _outhits
    (if (== (`.HitActor` (`GameplayStatics.BreakHitResult` _array_element)) (`self.Array Element Hit Actor`))
      (break)
      (else
        (bind _output_get (set `self.Array Element Hit Actor` (`.HitActor` (`GameplayStatics.BreakHitResult` _array_element))))
        (`self.TryToPickUp` _output_get)
        (message `ISCombatInterface.ApplyDamageToTarget` (`self.GetOwner`) _output_get)))))

(event `ISEquipableInterface.EndAbilityActivate`
  (`self.Array Element Hit Actor`
    (:`then`
      (set `self.Array Element Hit Actor` null))
    (:`else`)))

(fn `TryToPickUp`
  (params (InActor :type "Actor Object Reference"))
  (if (`KismetSystemLibrary.DoesImplementInterface` InActor "/Script/IslandSurvival.ISCollectibleInterface")
    (bind _returnvalue (message `ISCollectibleInterface.GetTargetClass` InActor))
    (switch `ECollectibleClass` _returnvalue
      (:`Corpse`
        (bind _output_get (set `self.Array Element Hit Actor` InActor))
        (message `ISCollectibleInterface.CollectionExecution` _output_get (`self.GetOwner`) self)
        (return)))
    (else
      (return))))

(fn `UserConstructionScript`
  (`parent.UserConstructionScript`))