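; Harvestable palm tree, a large-item child class that topples when broken and gives hit feedback.
; On break, it enables physics on the harvest mesh, pushes it along the target actor's forward vector with a mass-scaled acceleration-change force, then destroys itself after a delay.
; CallMulticastDelegates triggers MulticastVFX, which spawns a scaled-down concrete destruction emitter and plays a hatchet hit sound at the tree's location.
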(event `self.EnableHarvestionBreak`
  (params (TargetActor :type "Actor Object Reference"))
  (`PrimitiveComponent.SetSimulatePhysics` (`self.HarvestStaticMesh`) true)
  (`PrimitiveComponent.AddForce` (`self.HarvestStaticMesh`) (* (`self.GetActorForwardVector` TargetActor) (`PrimitiveComponent.GetMass` (`self.HarvestStaticMesh`))) "None" true)
  (`KismetSystemLibrary.Delay` 10.0)
  (`self.K2_DestroyActor`))

(event `self.CallMulticastDelegates`
  (`self.MulticastVFX`))

(event `MulticastVFX`
  (bind _returnvalue (`self.K2_GetActorLocation`))
  (`GameplayStatics.SpawnEmitterAtLocation` "/Game/Realistic_Starter_VFX_Pack_Vol2/Particles/Destruction/P_Destruction_Concrete.P_Destruction_Concrete" _returnvalue (struct) (0.1 0.1 0.1))
  (`GameplayStatics.PlaySoundAtLocation` "/Game/EasyBuildingSystem/Audio/Sounds/Interactions/Chopping/SC_Hatchet_Hit.SC_Hatchet_Hit" _returnvalue (struct) 1.0 1.0 0.0 null null null null))

(fn `UserConstructionScript`)