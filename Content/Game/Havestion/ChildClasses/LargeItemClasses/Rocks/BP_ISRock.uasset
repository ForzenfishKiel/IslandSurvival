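; Harvestable rock, a child large-item Blueprint that gives feedback when hit and shatters when broken.
; Hits route through CallMulticastDelegates to MulticastVFX, which spawns concrete debris particles and a pickaxe sound at the rock.
; EnableHarvestionBreak routes to MulticastEveryone, which spawns BP_DestroySystem, plays a 2D break sound and sets the GeometryCollection to WorldDynamic.
; The broken rock destroys itself after a short delay.
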(event `self.EnableHarvestionBreak`
  (params (TargetActor :type "Actor Object Reference"))
  ;[0 0.5432 1] BrokeAndMulticast
  (`self.MulticastEveryone`))

(event `MulticastEveryone`
  ;[0 0.5432 1] BrokeAndMulticast
  (`|SpawnActorFromClass` "/Game/Game/Havestion/BP_DestroySystem.BP_DestroySystem_C" (`KismetMathLibrary.MakeTransform` (`self.K2_GetActorLocation`)) "Undefined" "MultiplyWithRoot" null null)
  (`GameplayStatics.PlaySound2D` "/Game/Game/Havestion/ChildClasses/LargeItemClasses/Rocks/VFX/SC_RockBroke.SC_RockBroke" 1.0 1.0 0.0 null null)
  (`PrimitiveComponent.SetCollisionObjectType` (`self.GeometryCollection`) "ECC_WorldDynamic")
  (`KismetSystemLibrary.Delay` 8.0)
  (`self.K2_DestroyActor`))

(event `self.CallMulticastDelegates`
  ;[0 1 0.3016] 播放视觉效果
  (`self.MulticastVFX`))

(event `MulticastVFX`
  (bind _returnvalue (`self.K2_GetActorLocation`))
  ;[0 1 0.3016] 播放视觉效果
  (`GameplayStatics.SpawnEmitterAtLocation` "/Game/Realistic_Starter_VFX_Pack_Vol2/Particles/Destruction/P_Destruction_Concrete.P_Destruction_Concrete" _returnvalue (struct) (0.1 0.1 0.1))
  (`GameplayStatics.PlaySoundAtLocation` "/Game/EasyBuildingSystem/Audio/Sounds/Interactions/Mining/SC_Pickaxe_Hit.SC_Pickaxe_Hit" _returnvalue (struct) 1.0 1.0 0.0 null null null null))

(fn `UserConstructionScript`)