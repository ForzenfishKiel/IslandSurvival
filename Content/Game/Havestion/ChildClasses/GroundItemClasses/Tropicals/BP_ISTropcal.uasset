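; BP_ISTropcal is a tropical ground-item child class in the harvesting system that handles hit feedback and breakage.
; CallMulticastDelegates triggers MulticastEveryOne, which spawns a concrete destruction particle and a tropical hit sound at the actor's location.
; EnableHarvestionBreak turns on mesh physics, pushes it along the target actor's forward vector with a mass-scaled force, then destroys the actor after a short delay.
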(event `self.CallMulticastDelegates`
  ;[0.09237 0.1206 1] 播放VFX
  (`self.MulticastEveryOne`))

(event `MulticastEveryOne`
  (bind _returnvalue (`self.K2_GetActorLocation`))
  ;[0.09237 0.1206 1] 播放VFX
  (`GameplayStatics.SpawnEmitterAtLocation` "/Game/Realistic_Starter_VFX_Pack_Vol2/Particles/Destruction/P_Destruction_Concrete.P_Destruction_Concrete" _returnvalue)
  (`GameplayStatics.PlaySoundAtLocation` "/Game/Game/Havestion/ChildClasses/GroundItemClasses/Tropicals/VFX/SC_TropicalHit.SC_TropicalHit" _returnvalue (struct) 1.0 1.0 0.0 null null null null))

(event `self.EnableHarvestionBreak`
  (params (TargetActor :type "Actor Object Reference"))
  (`PrimitiveComponent.SetSimulatePhysics` (`self.HarvestStaticMesh`) true)
  (`PrimitiveComponent.AddForce` (`self.HarvestStaticMesh`) (* (`self.GetActorForwardVector` TargetActor) (`PrimitiveComponent.GetMass` (`self.HarvestStaticMesh`))) "None" true)
  (`KismetSystemLibrary.Delay` 3.0)
  (`self.K2_DestroyActor`))

(fn `UserConstructionScript`
  (`parent.UserConstructionScript`))