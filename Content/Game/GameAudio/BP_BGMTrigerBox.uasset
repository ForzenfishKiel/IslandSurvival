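; BP_BGMTrigerBox is a trigger volume that starts and stops the LevelDefault background music for players inside it.
; Eight seconds after BeginPlay, it fades in music for players already overlapping its collision component.
; Entering restarts the track with fades, while exiting stops it immediately.
; Actors are filtered by ISPlayerInterface, and music calls go through the object returned by GetSourceCharacterMessage.
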(event `self.ReceiveBeginPlay`
  (`KismetSystemLibrary.Delay` 8.0)
  (for _array_element (`PrimitiveComponent.GetOverlappingActors` (`self.CollisionComponent`) null)
    (if (`KismetSystemLibrary.DoesImplementInterface` _array_element "/Script/IslandSurvival.ISPlayerInterface")
      (bind _returnvalue (message `ISPlayerInterface.GetSourceCharacter` _array_element))
      (`ISCharacter.PlayBGM` _returnvalue "LevelDefault" 3.0))))

(event `self.ReceiveActorBeginOverlap`
  (params (OtherActor :type "Actor Object Reference"))
  (`/Engine/EditorBlueprintResources/StandardMacros.IsValid` OtherActor
    (:`Is Valid`
      (if (`KismetSystemLibrary.DoesImplementInterface` OtherActor "/Script/IslandSurvival.ISPlayerInterface")
        (bind _returnvalue (message `ISPlayerInterface.GetSourceCharacter` OtherActor))
        (`/Engine/EditorBlueprintResources/StandardMacros.IsValid` _returnvalue
          (:`Is Valid`
            (`ISCharacter.StopBGM` _returnvalue "LevelDefault" 3.0)
            (`ISCharacter.PlayBGM` _returnvalue "LevelDefault" 2.0)))))))

(event `self.CollisionComponent.OnComponentEndOverlap`
  (params (OverlappedComponent :type "PrimitiveComponent Object Reference") (OtherActor :type "Actor Object Reference") (OtherComp :type "PrimitiveComponent Object Reference") (OtherBodyIndex :type Integer))
  (`/Engine/EditorBlueprintResources/StandardMacros.IsValid` OtherActor
    (:`Is Valid`
      (if (`KismetSystemLibrary.DoesImplementInterface` OtherActor "/Script/IslandSurvival.ISPlayerInterface")
        (bind _returnvalue (message `ISPlayerInterface.GetSourceCharacter` OtherActor))
        (`/Engine/EditorBlueprintResources/StandardMacros.IsValid` _returnvalue
          (:`Is Valid`
            (`ISCharacter.StopBGM` _returnvalue "LevelDefault" 0.0)))))))

(fn `UserConstructionScript`)