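; BP_Zone is a procedural zone that spawns random wildlife the first time a player enters its box.
; On the server, an overlapping ISPlayerInterface actor triggers a one-time spawn of a few deer and wolves, stored in an AI array.
; FindSpawnLocation line-traces from a random point in scale-sized bounds, retrying until it hits, and animals spawn above the hit.
; The trace end adds coordinates derived from that point, and debug lines draw persistently.
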(event `self.Box.OnComponentBeginOverlap`
  (params (OverlappedComponent :type "PrimitiveComponent Object Reference") (OtherActor :type "Actor Object Reference") (OtherComp :type "PrimitiveComponent Object Reference") (OtherBodyIndex :type Integer) (bFromSweep :type Boolean) (SweepResult :type "HitResult Structure (by ref)"))
  (`/Engine/EditorBlueprintResources/ActorMacros.Switch Has Authority`
    (:`Authority`
      (if (`KismetSystemLibrary.DoesImplementInterface` OtherActor "/Script/IslandSurvival.ISPlayerInterface")
        (`self.SpawnAiEvent`)))))

(event `self.Box.OnComponentEndOverlap`
  (params (OverlappedComponent :type "PrimitiveComponent Object Reference") (OtherActor :type "Actor Object Reference") (OtherComp :type "PrimitiveComponent Object Reference") (OtherBodyIndex :type Integer)))

(event `SpawnAiEvent`
  ;[0 0.3942 1] 随机生成AI
  (if (not (`self.bAISpawn`))
    (set `self.bAISpawn` true)
    (for _ (range 1 (+ (`KismetMathLibrary.RandomIntegerInRange` 1 3) 1))
      (bind (_bblockinghit _location) (`self.FindSpawnLocation` :!label _label))
      (if _bblockinghit
        (bind _returnvalue (`|SpawnActorFromClass` "/Game/Game/Character/Enemies/Animals/Deers/BP_Deer.BP_Deer_C" (`KismetMathLibrary.MakeTransform` (+ _location (0.0 0.0 200.0))) "Undefined" "MultiplyWithRoot" null null))
        (`KismetArrayLibrary.Array_Add` (`self.AI`) _returnvalue)
        (else
          (goto _label))))
    (for _ (range 1 (+ (`KismetMathLibrary.RandomIntegerInRange` 1 2) 1))
      (bind (_bblockinghit_2 _location_2) (`self.FindSpawnLocation` :!label _label_2))
      (if _bblockinghit_2
        (bind _returnvalue_2 (`|SpawnActorFromClass` "/Game/Game/Character/Enemies/Animals/Wolf/BP_ISWolf.BP_ISWolf_C" (`KismetMathLibrary.MakeTransform` (+ _location_2 (0.0 0.0 200.0))) "Undefined" "MultiplyWithRoot" null null))
        (`KismetArrayLibrary.Array_Add` (`self.AI`) _returnvalue_2)
        (else
          (goto _label_2))))))

(fn `FindSpawnLocation`
  (returns (bBlockingHit :type Boolean) (Location :type "Vector Structure"))
  (bind (_returnvalue_location _returnvalue_rotation _returnvalue_scale) (`KismetMathLibrary.BreakTransform` (`self.GetTransform`)))
  (bind (_randompoint_x _randompoint_y) (`KismetMathLibrary.BreakVector` (`self.RandomPoint`)))
  (bind (_returnvalue_x _returnvalue_y _returnvalue_z) (`KismetMathLibrary.BreakVector` (* (`self.RandomPoint`) (`self.TraceDistance`))))
  (set `self.RandomPoint` (`KismetMathLibrary.RandomPointInBoundingBox` (`self.K2_GetActorLocation`) (* _returnvalue_scale 30.0)))
  (bind _outhit (`KismetSystemLibrary.LineTraceSingle` (`self.RandomPoint`) (+ (`self.RandomPoint`) (`KismetMathLibrary.MakeVector` _randompoint_x _randompoint_y _returnvalue_z)) "TraceTypeQuery13" true (`|MakeArray` self :!type "Actor Object Reference") "Persistent"))
  (bind (_bblockinghit _binitialoverlap _time _distance _location) (`GameplayStatics.BreakHitResult` _outhit))
  (return _bblockinghit _location))

(fn `UserConstructionScript`)